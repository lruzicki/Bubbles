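; BP_Actor is an actor that travels along the spline of a BP_Path actor found in the level.
; On BeginPlay it looks up that path with GetActorOfClass, stores it and calls StartMoving.
; A Timeline alpha interpolates distance from zero to the spline's length, and each update sets the actor's world location and rotation from the spline transform at that distance.
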(event Custom|Start%20Moving
  (bind _alpha (Timeline|Timeline Play)
    (:Update
      (Transformation|SetActorLocationAndRotation (.location (Spline|GetTransformatDistanceAlongSpline (Variables|/Game/MatizRuch/BP_Path.BP_Path_C|GetSpline (Variables|Default|GetPath)) (Math|Float|Lerp 0.0 (Spline|GetSplineLength (Variables|/Game/MatizRuch/BP_Path.BP_Path_C|GetSpline (Variables|Default|GetPath))) _alpha) "World" false)) (.rotation (Spline|GetTransformatDistanceAlongSpline (Variables|/Game/MatizRuch/BP_Path.BP_Path_C|GetSpline (Variables|Default|GetPath)) (Math|Float|Lerp 0.0 (Spline|GetSplineLength (Variables|/Game/MatizRuch/BP_Path.BP_Path_C|GetSpline (Variables|Default|GetPath))) _alpha) "World" false))))))

(event EventBeginPlay
  (bind _returnvalue (Actor|GetActorOfClass "/Game/MatizRuch/BP_Path.BP_Path_C"))
  (Variables|Default|SetPath _returnvalue)
  (CallFunction|StartMoving))

(event Collision|EventActorBeginOverlap
  (params (OtherActor :type Actor%20Object%20Reference)))

(event EventTick
  (params (DeltaSeconds :type Float%20%28single-precision%29)))

(fn ConstructionScript)