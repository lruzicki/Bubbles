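; Security guard AI character that patrols, chases the player on sight and restarts the level on a catch.
; Tick derives a distance-based danger value, flags GameMode chasing when Points changes while watched, and schedules patrols when unseen.
; PawnSensing starts the chase, with a retriggerable delay clearing sight.
; Catching turns player and camera toward the guard, plays a montage, fades out and reloads the level.
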(event OnSeePawn(PawnSensing)
  (params (Pawn :type Pawn%20Object%20Reference))
  ;[0.15 0.15 0.15 0.5] Mechanika na gonienie usera
  (bind _asbp_third_person_character (Utilities|Casting|CastToBP_ThirdPersonCharacter Pawn))
  (bind _asbp_third_person_game_mode (Utilities|Casting|CastToBP_ThirdPersonGameMode (Game|GetGameMode)))
  (if (not (and false (Variables|/Game/ThirdPerson/Blueprints/BP_ThirdPersonGameMode.BP_ThirdPersonGameMode_C|GetchasingPlayer _asbp_third_person_game_mode)))
    (Utilities|FlowControl|Sequence
      (:then_0
        (Variables|Default|SetIsSeeingPlayer true)
        (AI|AIMoveTo self "0, 0, 0" _asbp_third_person_character 5.0 false
          (:OnSuccess
            (CallFunction|CatchPlayer))))
      (:then_1
        (Utilities|FlowControl|RetriggerableDelay 0.3)
        (Variables|Default|SetIsSeeingPlayer false)))))

(event Custom|CatchPlayer
  (bind _returnvalue (Game|GetPlayerController 0))
  (Variables|Default|SetisCaught true)
  (bind _asbp_third_person_character (Utilities|Casting|CastToBP_ThirdPersonCharacter (Game|GetPlayerCharacter 0)))
  (if (Variables|Default|GetisCaught)
    (Utilities|FlowControl|Delay 0.001)
    (Transformation|SetActorRotation _asbp_third_person_character (Math|Interpolation|RInterpTo (Transformation|GetActorRotation _asbp_third_person_character) (Math|Rotator|FindLookatRotation (Transformation|GetActorLocation _asbp_third_person_character) (Transformation|GetActorLocation)) (Utilities|Time|GetWorldDeltaSeconds) 5.0))
    (Pawn|SetControlRotation _returnvalue (Math|Interpolation|RInterpTo (Pawn|GetControlRotation _returnvalue :!class /Script/Engine.Controller) (Math|Rotator|FindLookatRotation (Transformation|GetActorLocation _asbp_third_person_character) (Transformation|GetActorLocation)) (Utilities|Time|GetWorldDeltaSeconds) 5.0))
    (CallFunction|RotationLoop)
    (Utilities|FlowControl|DoOnce false :!label _label
      (:Completed
        (Utilities|FlowControl|Sequence
          (:then_0
            (Animation|PlayAnimMontage "/Game/Characters/Mannequins/Animations/Manny/CatchPlayer.CatchPlayer" 1.0 "None")
            (Utilities|FlowControl|Delay 1.0)
            (CameraFades|StartCameraFade :self (Game|GetPlayerCameraManager 0) :ToAlpha 1.0 :Duration 2.0 :bShouldFadeAudio true :bHoldWhenFinished true)
            (Utilities|FlowControl|Delay 2.1)
            (bind _returnvalue_2 (Game|GetCurrentLevelName true))
            (Game|OpenLevel(byName) (Utilities|String|StringToName _returnvalue_2)))
          (:then_1
            (Utilities|FlowControl|Delay 0.5)
            (Variables|Default|SetisCaught false)
            (goto _label Reset)))))))

(event Custom|RotationLoop
  (bind _returnvalue (Game|GetPlayerController 0))
  (if (Variables|Default|GetisCaught)
    (Utilities|FlowControl|Delay 0.001)
    (Transformation|SetActorRotation (stale Custom|CatchPlayer _asbp_third_person_character) (Math|Interpolation|RInterpTo (Transformation|GetActorRotation (stale Custom|CatchPlayer _asbp_third_person_character)) (Math|Rotator|FindLookatRotation (Transformation|GetActorLocation (stale Custom|CatchPlayer _asbp_third_person_character)) (Transformation|GetActorLocation)) (Utilities|Time|GetWorldDeltaSeconds) 5.0))
    (Pawn|SetControlRotation _returnvalue (Math|Interpolation|RInterpTo (Pawn|GetControlRotation _returnvalue :!class /Script/Engine.Controller) (Math|Rotator|FindLookatRotation (Transformation|GetActorLocation (stale Custom|CatchPlayer _asbp_third_person_character)) (Transformation|GetActorLocation)) (Utilities|Time|GetWorldDeltaSeconds) 5.0))
    (CallFunction|RotationLoop)
    (Utilities|FlowControl|DoOnce false :!label _label
      (:Completed
        (Utilities|FlowControl|Sequence
          (:then_0
            (Animation|PlayAnimMontage "/Game/Characters/Mannequins/Animations/Manny/CatchPlayer.CatchPlayer" 1.0 "None")
            (Utilities|FlowControl|Delay 1.0)
            (CameraFades|StartCameraFade :self (Game|GetPlayerCameraManager 0) :ToAlpha 1.0 :Duration 2.0 :bShouldFadeAudio true :bHoldWhenFinished true)
            (Utilities|FlowControl|Delay 2.1)
            (bind _returnvalue_2 (Game|GetCurrentLevelName true))
            (Game|OpenLevel(byName) (Utilities|String|StringToName _returnvalue_2)))
          (:then_1
            (Utilities|FlowControl|Delay 0.5)
            (Variables|Default|SetisCaught false)
            (goto _label Reset)))))))

(event Custom|Guard
  ;[0.15 0.15 0.15 0.5] Mechanika na patrolowanie konktetnych lokacji
  (Variables|/Script/Engine.CharacterMovementComponent|SetMaxWalkSpeed (Variables|Character|GetCharacterMovement) 155.0)
  (AI|AIMoveTo self (Utilities|Array|Get(acopy) (Variables|Default|GetPatrolLocation) (Variables|Default|GetLocations)) 0 5.0 false
    (:OnSuccess
      (Utilities|FlowControl|Delay (Math|Random|RandomFloatinRange 1.0 3.0))
      (CallFunction|Guard)
      (Math|Integer|IncrementInt (Variables|Default|GetLocations)
        (:%20%20
          (if (== (Variables|Default|GetLocations) 4)
            _))))))

(event EventTick
  (params (DeltaSeconds :type Float%20%28single-precision%29))
  ;[0.15 0.15 0.15 0.5] Reset akcji - jak nie widzi usera to robi akcje Guard - czyli wartuje xD
  (if (Variables|Default|GetIsSeeingPlayer)
    (Variables|Default|SetguardLocalDanger (+ (* (Math|Float|Absolute(Float) (Math|Vector|Distance(Vector) (Transformation|GetActorLocation) (Transformation|GetActorLocation (Game|GetPlayerCharacter 0)))) 23.5) 2.5e+03))
    (else
      (Variables|Default|SetguardLocalDanger 0.0)))
  (Development|PrintString "Hello" false false "(R=1.000000,G=0.032495,B=0.873306,A=1.000000)")
  ;[0.15 0.15 0.15 0.5] Don't follow player if not seen throwing cart
  (bind _asbp_third_person_game_mode (Utilities|Casting|CastToBP_ThirdPersonGameMode (Game|GetGameMode)))
  (if (and (!= (Variables|/Game/ThirdPerson/Blueprints/BP_ThirdPersonGameMode.BP_ThirdPersonGameMode_C|Getpoints _asbp_third_person_game_mode) (Variables|Default|GetpreviousPoints)) (Variables|Default|GetIsSeeingPlayer))
    (bind _asbp_third_person_game_mode_2 (Utilities|Casting|CastToBP_ThirdPersonGameMode (Game|GetGameMode)))
    (Variables|Default|SetpreviousPoints (Math|Conversions|ToBoolean(Integer) (Variables|/Game/ThirdPerson/Blueprints/BP_ThirdPersonGameMode.BP_ThirdPersonGameMode_C|Getpoints _asbp_third_person_game_mode_2)))
    (Variables|/Game/ThirdPerson/Blueprints/BP_ThirdPersonGameMode.BP_ThirdPersonGameMode_C|SetchasingPlayer _asbp_third_person_game_mode_2 true)
    (else
      (bind _asbp_third_person_game_mode_3 (Utilities|Casting|CastToBP_ThirdPersonGameMode (Game|GetGameMode)))
      (Variables|Default|SetpreviousPoints (Math|Conversions|ToBoolean(Integer) (Variables|/Game/ThirdPerson/Blueprints/BP_ThirdPersonGameMode.BP_ThirdPersonGameMode_C|Getpoints _asbp_third_person_game_mode_3)))))
  (if (not (Variables|Default|GetIsSeeingPlayer))
    (Utilities|FlowControl|Delay (Math|Random|RandomFloatinRange 1.0 2.0))
    (CallFunction|Guard)))

(fn ConstructionScript)