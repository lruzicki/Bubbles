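; BP_cart is a cart the third-person player grabs or releases with E after entering its overlap.
; While held, Tick turns off physics and places the mesh ahead of the player, matching rotation with a yaw offset and using a downward trace for height.
; Released, it simulates physics, and hits with enough upward velocity play a debounced crash sound.
; Looping Tick logic also raises audio volume while pushed and mutes it when the player stops.
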(event EventBeginPlay
  (bind _asbp_third_person_character (Utilities|Casting|CastToBP_ThirdPersonCharacter (Game|GetPlayerCharacter 0)))
  (Variables|Default|Setplayer _asbp_third_person_character)
  (Variables|Default|SetplayerInside false)
  (Variables|Default|SetmatchPlayerPosition false)
  (Physics|SetEnableGravity (Variables|Default|GetStaticMesh) true)
  (Input|EnableInput 0)
  (Physics|SetSimulatePhysics (Variables|Default|GetStaticMesh) false)
  (Audio|Components|Audio|Play (Variables|Default|GetAudio) 0.0))

(event Collision|EventActorBeginOverlap
  (params (OtherActor :type Actor%20Object%20Reference))
  (Utilities|Casting|CastToBP_ThirdPersonCharacter OtherActor)
  (Variables|Default|SetplayerInside true))

(event Collision|EventHit
  (params (MyComp :type Primitive%20Component%20Object%20Reference) (Other :type Actor%20Object%20Reference) (OtherComp :type Primitive%20Component%20Object%20Reference) (bSelfMoved :type Boolean) (HitLocation :type Vector :default "0, 0, 0") (HitNormal :type Vector :default "0, 0, 0") (NormalImpulse :type Vector :default "0, 0, 0") (Hit :type Hit%20Result%20Structure%20%28by%20ref%29))
  (if (not (Variables|Default|GetmatchPlayerPosition))
    (bind _returnvalue (Physics|GetPhysicsLinearVelocity (Variables|Default|GetStaticMesh) "None"))
    (Math|Float|CompareFloat (.Z (Math|Vector|BreakVector _returnvalue)) 2.0
      (:>
        (Utilities|FlowControl|DoOnce false :!label _label
          (:Completed
            (Audio|PlaySoundatLocation "/Game/Sounds/CartCrash.CartCrash" HitLocation "0, 0, 0" 1.0 1.0 0.0 "/Game/Sounds/CartCrashAttenuation.CartCrashAttenuation" 0 0 0)
            (Utilities|FlowControl|Delay 0.2)
            (goto _label Reset)))))))

(event Collision|EventActorEndOverlap
  (params (OtherActor :type Actor%20Object%20Reference))
  (Variables|Default|SetplayerInside false))

(event EventTick
  (params (DeltaSeconds :type Float%20%28single-precision%29))
  (bind _player (Variables|Default|Getplayer))
  (bind _player_2 (Variables|Default|Getplayer))
  (bind _player_3 (Variables|Default|Getplayer))
  (bind _returnvalue (Transformation|GetActorRotation _player_2))
  (bind _returnvalue_2 (Transformation|GetActorLocation _player))
  (bind _returnvalue_3 (Transformation|GetActorLocation _player_3))
  (bind _rootcomponent (Variables|/Script/Engine.Actor|GetRootComponent _player))
  (bind (_roll _pitch _yaw) (Math|Rotator|BreakRotator _returnvalue))
  (bind _returnvalue_4 (Math|Vector|GetForwardVector _rootcomponent))
  (bind _returnvalue_5 (* _returnvalue_4 "100.000000,100.000000,100.000000"))
  (bind _returnvalue_6 (+ _returnvalue_2 _returnvalue_5))
  (bind (_x _y) (Math|Vector|BreakVector _returnvalue_6))
  (Utilities|FlowControl|Sequence
    (:then_0
      (if (Variables|Default|GetmatchPlayerPosition)
        (Utilities|FlowControl|Sequence
          (:then_0
            (Physics|SetSimulatePhysics (Variables|Default|GetStaticMesh) false)
            (Transformation|SetRelativeRotation (Variables|Default|GetStaticMesh) (Math|Rotator|MakeRotator _roll _pitch (+ _yaw 2.7e+02)) false false)
            (bind _outhit (Collision|LineTraceByChannel (+ _returnvalue_3 "0.000000,0.000000,200.000000") (- _returnvalue_3 "0.000000,0.000000,1500.000000") "TraceTypeQuery1" false 0 "None"))
            (Transformation|SetRelativeLocation (Variables|Default|GetStaticMesh) (Math|Vector|MakeVector _x _y (.Z (Math|Vector|BreakVector (.ImpactPoint (Collision|BreakHitResult _outhit))))) false false)))
        (else
          (Physics|SetSimulatePhysics (Variables|Default|GetStaticMesh) true))))
    (:then_1
      (Audio|Components|Audio|SetVolumeMultiplier (Variables|Default|GetAudio) (Variables|Default|GetmusicVol) :!class /Script/Engine.AudioComponent)
      (if (Utilities|Operators|EqualEqual (Variables|Default|GetprevPos) (Transformation|GetActorLocation (Variables|Default|Getplayer)) 0.0)
        (Variables|Default|SetmusicVol 0.0)
        (elif (Variables|Default|GetmatchPlayerPosition)
          (Variables|Default|SetmusicVol 1.0))))
    (:then_2
      (Variables|Default|SetprevPos (Transformation|GetActorLocation (Variables|Default|Getplayer))))))

(event Input|KeyboardEvents|E
  (params (Key :type Key%20Structure :default "None"))
  (:Pressed
    (if (Variables|Default|GetmatchPlayerPosition)
      (Variables|Default|SetmatchPlayerPosition false)
      (elif (Variables|Default|GetplayerInside)
        (Variables|Default|SetmatchPlayerPosition true)))))

(fn ConstructionScript)